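; BP_Holst is an interactable canvas ("holst") that shows a progressively updated picture alongside animated on-screen guide widgets.
; Each Interact, throttled by a DoOnce that resets after a short delay, increments Uses and calls NewPic to swap the mesh material and replace the current guide.
; Once Uses maxes out, the next interaction destroys Cube, reveals Cube1, disables actor collision and briefly shows the final guide.
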(event Custom|NewPic
  (bind _uses (Variables|Default|GetUses))
  (bind _cube (Variables|Default|GetCube))
  (Utilities|FlowControl|Sequence
    (:then_0
      (if (== _uses 1)
        (Rendering|Material|SetMaterial _cube 0 "/Game/Materials/первая_версия_Mat.первая_версия_Mat")
        (bind _returnvalue (UserInterface|CreateWidget "/Game/Blueprints/UI/UI_Guide2.UI_Guide2_C"))
        (UserInterface|Viewport|AddtoViewport _returnvalue 0)
        (UserInterface|Animation|PlayAnimation _returnvalue (Variables|/Game/Blueprints/UI/UI_Guide2.UI_Guide2_C|GetNewAnimation _returnvalue) 0.0 1 "Forward" 1.0 false)
        (Widget|RemovefromParent (stale EventBeginPlay _returnvalue))))
    (:then_1
      (if (== _uses 2)
        (Rendering|Material|SetMaterial _cube 0 "/Game/Materials/вторая_версия_Mat.вторая_версия_Mat")
        (bind _returnvalue_2 (UserInterface|CreateWidget "/Game/Blueprints/UI/UI_Guide3.UI_Guide3_C"))
        (UserInterface|Viewport|AddtoViewport _returnvalue_2 0)
        (UserInterface|Animation|PlayAnimation _returnvalue_2 (Variables|/Game/Blueprints/UI/UI_Guide3.UI_Guide3_C|GetNewAnimation _returnvalue_2) 0.0 1 "Forward" 1.0 false)
        (Widget|RemovefromParent _returnvalue)))
    (:then_2
      (if (== _uses 3)
        (Rendering|Material|SetMaterial _cube 0 "/Game/Materials/третья_версия_Mat.третья_версия_Mat")
        (bind _returnvalue_3 (UserInterface|CreateWidget "/Game/Blueprints/UI/UI_Guide4.UI_Guide4_C"))
        (UserInterface|Viewport|AddtoViewport _returnvalue_3 0)
        (UserInterface|Animation|PlayAnimation _returnvalue_3 (Variables|/Game/Blueprints/UI/UI_Guide4.UI_Guide4_C|GetNewAnimation _returnvalue_3) 0.0 1 "Forward" 1.0 false)
        (Widget|RemovefromParent _returnvalue_2)))
    (:then_3
      (if (== _uses 4)
        (Rendering|Material|SetMaterial _cube 0 "/Game/Materials/четвертая_версия_Mat.четвертая_версия_Mat")
        (bind _returnvalue_4 (UserInterface|CreateWidget "/Game/Blueprints/UI/UI_Guide4.UI_Guide4_C"))
        (UserInterface|Viewport|AddtoViewport _returnvalue_4 0)
        (UserInterface|Animation|PlayAnimation _returnvalue_4 (Variables|/Game/Blueprints/UI/UI_Guide4.UI_Guide4_C|GetNewAnimation _returnvalue_4) 0.0 1 "Forward" 1.0 false)
        (Widget|RemovefromParent _returnvalue_3)))
    (:then_4
      (if (== _uses 5)
        (Rendering|Material|SetMaterial (Variables|Default|GetCube1) 0 "/Game/Materials/четвертая_версия_Mat.четвертая_версия_Mat")
        (bind _returnvalue_5 (UserInterface|CreateWidget "/Game/Blueprints/UI/UI_Guide4.UI_Guide4_C"))
        (UserInterface|Viewport|AddtoViewport _returnvalue_5 0)
        (UserInterface|Animation|PlayAnimation _returnvalue_5 (Variables|/Game/Blueprints/UI/UI_Guide4.UI_Guide4_C|GetNewAnimation _returnvalue_5) 0.0 1 "Forward" 1.0 false)
        (Widget|RemovefromParent _returnvalue_4)))))

(event EventBeginPlay
  (bind _returnvalue (UserInterface|CreateWidget "/Game/Blueprints/UI/UI_Guide1.UI_Guide1_C"))
  (UserInterface|Viewport|AddtoViewport _returnvalue 0)
  (UserInterface|Animation|PlayAnimation _returnvalue (Variables|/Game/Blueprints/UI/UI_Guide1.UI_Guide1_C|GetNewAnimation _returnvalue) 0.0 1 "Forward" 1.0 false))

(event EventInteract
  (Utilities|FlowControl|DoOnce false :!label _label
    (:Completed
      (Utilities|FlowControl|Sequence
        (:then_0
          (if (>= (Variables|Default|GetUses) 5)
            (Components|DestroyComponent (Variables|Default|GetCube))
            (Rendering|SetVisibility (Variables|Default|GetCube1) true false)
            (Collision|SetActorEnableCollision false)
            (bind _returnvalue (UserInterface|CreateWidget "/Game/Blueprints/UI/UI_Guide5.UI_Guide5_C"))
            (UserInterface|Viewport|AddtoViewport _returnvalue 0)
            (UserInterface|Animation|PlayAnimation _returnvalue (Variables|/Game/Blueprints/UI/UI_Guide5.UI_Guide5_C|GetNewAnimation _returnvalue) 0.0 1 "Forward" 1.0 false)
            (Widget|RemovefromParent (stale Custom|NewPic _returnvalue_5))
            (Utilities|FlowControl|Delay 1e+01)
            (Widget|RemovefromParent _returnvalue)
            (else
              (Math|Integer|IncrementInt (Variables|Default|GetUses)
                (:%20%20
                  (CallFunction|NewPic))))))
        (:then_1
          (Utilities|FlowControl|Delay 1.0)
          (goto _label Reset))))))

(fn ConstructionScript
  (|CallParentFunction))