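; Interactable toilet stall door whose response depends on whether the player has obtained toilet paper.
; Without paper, Interact hides the first-person character, blends to the door's view, enables click events and spawns the paper, throttled by a resettable DoOnce.
; With paper, it activates the level's valve, removes the MAn component and swings the door via a timeline.
; Leave restores the character, input and player view.
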(event Custom|Leave
  (bind _returnvalue (Game|GetPlayerCharacter 0))
  (bind _returnvalue_2 (Game|GetPlayerController 0))
  (bind _asbp_first_person_character (Utilities|Casting|CastToBP_FirstPersonCharacter _returnvalue))
  (Rendering|SetActorHiddenInGame _asbp_first_person_character false)
  (Input|EnableInput _returnvalue _returnvalue_2)
  (Game|Player|SetViewTargetwithBlend _returnvalue_2 _returnvalue 0.25 "VTBlend_Linear" 0.0 false))

(event EventInteract
  (bind _returnvalue (Game|GetPlayerController 0))
  (bind _paper (Variables|Default|GetPaper))
  (if (Variables|/Game/Blueprints/BP_ToiletPaper.BP_ToiletPaper_C|GetHave%20Toilet%20Paper (Variables|Default|GetPaper))
    (Default|ValveActivate (Variables|Default|GetValve))
    (Components|DestroyComponent (Variables|Default|GetMAn))
    (bind _newtrack_0 (Timeline|Door%20Anim Play)
      (:Update
        (Transformation|SetRelativeRotation (Variables|Default|GetScene) (Math|Rotator|MakeRotator 0.0 0.0 _newtrack_0) false false)))
    (else
      (Class|WidgetBlueprintLibrary|SetFocustoGameViewport)
      (Utilities|FlowControl|DoOnce false :!label _label
        (:Completed
          (Utilities|FlowControl|Sequence
            (:then_0
              (bind _asbp_first_person_character (Utilities|Casting|CastToBP_FirstPersonCharacter (Game|GetPlayerCharacter 0)))
              (Rendering|SetActorHiddenInGame _asbp_first_person_character true)
              (Game|Player|SetViewTargetwithBlend _returnvalue self 0.25 "VTBlend_Linear" 0.0 false)
              (Rendering|SetVisibility (Variables|Default|GetWidget) false false)
              (Variables|/Script/Engine.PlayerController|SetbEnableClickEvents _returnvalue true)
              (Default|Spawn _paper)
              (Collision|SetActorEnableCollision _paper true))
            (:then_1
              (Utilities|FlowControl|Delay 1.0)
              (goto _label Reset))))))))

(event EventBeginPlay
  (bind _returnvalue (Actor|GetActorOfClass "/Game/Blueprints/BP_ToiletPaper.BP_ToiletPaper_C"))
  (Variables|Default|SetPaper _returnvalue)
  (bind _returnvalue_2 (Actor|GetActorOfClass "/Game/Blueprints/BP_Valve.BP_Valve_C"))
  (Variables|Default|SetValve _returnvalue_2))

(fn ConstructionScript
  (|CallParentFunction))