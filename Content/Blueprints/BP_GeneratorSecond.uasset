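; Interactive generator switch puzzle: interacting hides and disables the player, blends the view to the generator and enables mouse clicks.
; Four clickable switches toggle via FlipFlop and timelines, each shifting two gauge needles by its own offsets using MoveComponentTo.
; After each flip, Answer checks the switch states, not the needles; only switches 2 and 3 on solves it.
; Solving restores player view and input, disables the actor's collision and swings a door open.
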(event OnClicked(Switch01)
  (params (TouchedComponent :type Primitive%20Component%20Object%20Reference) (ButtonPressed :type Key%20Structure :default "None"))
  (Utilities|FlowControl|DoOnce false :!label _label
    (:Completed
      (Utilities|FlowControl|Sequence
        (:then_0
          (Input|SetInputModeGameandUI (Game|GetPlayerController 0) 0 "DoNotLock" true true)
          (Utilities|FlowControl|FlipFlop
            (:A
              (Variables|Default|SetSwitch01On true)
              (bind _value (Timeline|Switch%20Anim Play)
                (:Update
                  (Transformation|SetRelativeRotation (Variables|Default|GetSwitch01) (Math|Rotator|MakeRotator _value 0.0 0.0) false false))
                (:Finished
                  (CallFunction|Switch01)
                  (CallFunction|Answer))))
            (:B
              (Variables|Default|SetSwitch01On false)
              (Timeline|Switch%20Anim Reverse))))
        (:then_1
          (Utilities|FlowControl|Delay 0.3)
          (goto _label Reset))))))

(event OnClicked(Switch02)
  (params (TouchedComponent :type Primitive%20Component%20Object%20Reference) (ButtonPressed :type Key%20Structure :default "None"))
  (Utilities|FlowControl|DoOnce false :!label _label
    (:Completed
      (Utilities|FlowControl|Sequence
        (:then_0
          (Utilities|FlowControl|Delay 0.2)
          (goto _label Reset))
        (:then_1
          (Input|SetInputModeGameandUI (Game|GetPlayerController 0) 0 "DoNotLock" true true)
          (Utilities|FlowControl|FlipFlop
            (:A
              (Variables|Default|SetSwitch02On true)
              (bind _value (Timeline|Timeline Play)
                (:Update
                  (Transformation|SetRelativeRotation (Variables|Default|GetSwitch02) (Math|Rotator|MakeRotator _value 0.0 0.0) false false))
                (:Finished
                  (CallFunction|Switch02)
                  (CallFunction|Answer))))
            (:B
              (Variables|Default|SetSwitch02On false)
              (Timeline|Timeline Reverse))))))))

(event OnClicked(Switch03)
  (params (TouchedComponent :type Primitive%20Component%20Object%20Reference) (ButtonPressed :type Key%20Structure :default "None"))
  (Utilities|FlowControl|DoOnce false :!label _label
    (:Completed
      (Utilities|FlowControl|Sequence
        (:then_0
          (Utilities|FlowControl|Delay 0.2)
          (goto _label Reset))
        (:then_1
          (Input|SetInputModeGameandUI (Game|GetPlayerController 0) 0 "DoNotLock" true true)
          (Utilities|FlowControl|FlipFlop
            (:A
              (Variables|Default|SetSwitch03On true)
              (bind _value (Timeline|Timeline_0 Play)
                (:Update
                  (Transformation|SetRelativeRotation (Variables|Default|GetSwitch03) (Math|Rotator|MakeRotator _value 0.0 0.0) false false))
                (:Finished
                  (CallFunction|Switch03)
                  (CallFunction|Answer))))
            (:B
              (Variables|Default|SetSwitch03On false)
              (Timeline|Timeline_0 Reverse))))))))

(event OnClicked(Switch04)
  (params (TouchedComponent :type Primitive%20Component%20Object%20Reference) (ButtonPressed :type Key%20Structure :default "None"))
  (Utilities|FlowControl|DoOnce false :!label _label
    (:Completed
      (Utilities|FlowControl|Sequence
        (:then_0
          (Utilities|FlowControl|Delay 0.2)
          (goto _label Reset))
        (:then_1
          (Input|SetInputModeGameandUI (Game|GetPlayerController 0) 0 "DoNotLock" true true)
          (Utilities|FlowControl|FlipFlop
            (:A
              (Variables|Default|SetSwitch04On true)
              (bind _value (Timeline|Timeline_1 Play)
                (:Update
                  (Transformation|SetRelativeRotation (Variables|Default|GetSwitch04) (Math|Rotator|MakeRotator _value 0.0 0.0) false false))
                (:Finished
                  (CallFunction|Switch04)
                  (CallFunction|Answer))))
            (:B
              (Variables|Default|SetSwitch04On false)
              (Timeline|Timeline_1 Reverse))))))))

(event Custom|Switch%2001
  (bind _needle01 (Variables|Default|GetNeedle01))
  (bind _needle02 (Variables|Default|GetNeedle02))
  (bind _needle01_2 (Variables|Default|GetNeedle01))
  (bind _needle02_2 (Variables|Default|GetNeedle02))
  (if (Variables|Default|GetSwitch01On)
    (Utilities|FlowControl|Sequence
      (:then_0
        (Components|MoveComponentTo _needle01 (Variables|/Script/Engine.SceneComponent|GetRelativeLocation _needle01) (Math|Rotator|MakeRotator 1.8e+02 (- (.pitch (Variables|Default|GetNeedle01Relative)) -1e+01) 1.8e+02) false false 0.2 false)
        (Variables|Default|SetNeedle01Relative (Math|Rotator|MakeRotator 1.8e+02 (- (.pitch (Variables|Default|GetNeedle01Relative)) -1e+01) 1.8e+02)))
      (:then_1
        (Components|MoveComponentTo _needle02 (Variables|/Script/Engine.SceneComponent|GetRelativeLocation _needle02) (Math|Rotator|MakeRotator 1.8e+02 (- (.pitch (Variables|Default|GetNeedle02%20Relative)) -15.0) 1.8e+02) false false 0.2 false)
        (Variables|Default|SetNeedle02%20Relative (Math|Rotator|MakeRotator 1.8e+02 (- (.pitch (Variables|Default|GetNeedle02%20Relative)) -15.0) 1.8e+02))))
    (else
      (Utilities|FlowControl|Sequence
        (:then_0
          (Components|MoveComponentTo _needle01_2 (Variables|/Script/Engine.SceneComponent|GetRelativeLocation _needle01_2) (Math|Rotator|MakeRotator 1.8e+02 (- (.pitch (Variables|Default|GetNeedle01Relative)) 1e+01) 1.8e+02) false false 0.2 false)
          (Variables|Default|SetNeedle01Relative (Math|Rotator|MakeRotator 1.8e+02 (- (.pitch (Variables|Default|GetNeedle01Relative)) 1e+01) 1.8e+02)))
        (:then_1
          (Components|MoveComponentTo _needle02_2 (Variables|/Script/Engine.SceneComponent|GetRelativeLocation _needle02_2) (Math|Rotator|MakeRotator 1.8e+02 (- (.pitch (Variables|Default|GetNeedle02%20Relative)) 15.0) 1.8e+02) false false 0.2 false)
          (Variables|Default|SetNeedle02%20Relative (Math|Rotator|MakeRotator 1.8e+02 (- (.pitch (Variables|Default|GetNeedle02%20Relative)) 15.0) 1.8e+02)))))))

(event Custom|Switch%2004
  (bind _needle01 (Variables|Default|GetNeedle01))
  (bind _needle02 (Variables|Default|GetNeedle02))
  (bind _needle01_2 (Variables|Default|GetNeedle01))
  (bind _needle02_2 (Variables|Default|GetNeedle02))
  (if (Variables|Default|GetSwitch04On)
    (Utilities|FlowControl|Sequence
      (:then_0
        (Components|MoveComponentTo _needle01_2 (Variables|/Script/Engine.SceneComponent|GetRelativeLocation _needle01_2) (Math|Rotator|MakeRotator 1.8e+02 (- (.pitch (Variables|Default|GetNeedle01Relative)) 25.0) 1.8e+02) false false 0.2 false)
        (Variables|Default|SetNeedle01Relative (Math|Rotator|MakeRotator 1.8e+02 (- (.pitch (Variables|Default|GetNeedle01Relative)) 25.0) 1.8e+02)))
      (:then_1
        (Components|MoveComponentTo _needle02_2 (Variables|/Script/Engine.SceneComponent|GetRelativeLocation _needle02_2) (Math|Rotator|MakeRotator 1.8e+02 (- (.pitch (Variables|Default|GetNeedle02%20Relative)) -25.0) 1.8e+02) false false 0.2 false)
        (Variables|Default|SetNeedle02%20Relative (Math|Rotator|MakeRotator 1.8e+02 (- (.pitch (Variables|Default|GetNeedle02%20Relative)) -25.0) 1.8e+02))))
    (else
      (Utilities|FlowControl|Sequence
        (:then_0
          (Components|MoveComponentTo _needle01 (Variables|/Script/Engine.SceneComponent|GetRelativeLocation _needle01) (Math|Rotator|MakeRotator 1.8e+02 (- (.pitch (Variables|Default|GetNeedle01Relative)) -25.0) 1.8e+02) false false 0.2 false)
          (Variables|Default|SetNeedle01Relative (Math|Rotator|MakeRotator 1.8e+02 (- (.pitch (Variables|Default|GetNeedle01Relative)) -25.0) 1.8e+02)))
        (:then_1
          (Components|MoveComponentTo _needle02 (Variables|/Script/Engine.SceneComponent|GetRelativeLocation _needle02) (Math|Rotator|MakeRotator 1.8e+02 (- (.pitch (Variables|Default|GetNeedle02%20Relative)) 25.0) 1.8e+02) false false 0.2 false)
          (Variables|Default|SetNeedle02%20Relative (Math|Rotator|MakeRotator 1.8e+02 (- (.pitch (Variables|Default|GetNeedle02%20Relative)) 25.0) 1.8e+02)))))))

(event Custom|Switch%2002
  (bind _needle01 (Variables|Default|GetNeedle01))
  (bind _needle02 (Variables|Default|GetNeedle02))
  (bind _needle01_2 (Variables|Default|GetNeedle01))
  (bind _needle02_2 (Variables|Default|GetNeedle02))
  (if (Variables|Default|GetSwitch02On)
    (Utilities|FlowControl|Sequence
      (:then_0
        (Components|MoveComponentTo _needle01 (Variables|/Script/Engine.SceneComponent|GetRelativeLocation _needle01) (Math|Rotator|MakeRotator 1.8e+02 (- (.pitch (Variables|Default|GetNeedle01Relative)) -3e+01) 1.8e+02) false false 0.2 false)
        (Variables|Default|SetNeedle01Relative (Math|Rotator|MakeRotator 1.8e+02 (- (.pitch (Variables|Default|GetNeedle01Relative)) -3e+01) 1.8e+02)))
      (:then_1
        (Components|MoveComponentTo _needle02 (Variables|/Script/Engine.SceneComponent|GetRelativeLocation _needle02) (Math|Rotator|MakeRotator 1.8e+02 (- (.pitch (Variables|Default|GetNeedle02%20Relative)) -1e+01) 1.8e+02) false false 0.2 false)
        (Variables|Default|SetNeedle02%20Relative (Math|Rotator|MakeRotator 1.8e+02 (- (.pitch (Variables|Default|GetNeedle02%20Relative)) -1e+01) 1.8e+02))))
    (else
      (Utilities|FlowControl|Sequence
        (:then_0
          (Components|MoveComponentTo _needle01_2 (Variables|/Script/Engine.SceneComponent|GetRelativeLocation _needle01_2) (Math|Rotator|MakeRotator 1.8e+02 (- (.pitch (Variables|Default|GetNeedle01Relative)) 3e+01) 1.8e+02) false false 0.2 false)
          (Variables|Default|SetNeedle01Relative (Math|Rotator|MakeRotator 1.8e+02 (- (.pitch (Variables|Default|GetNeedle01Relative)) 3e+01) 1.8e+02)))
        (:then_1
          (Components|MoveComponentTo _needle02_2 (Variables|/Script/Engine.SceneComponent|GetRelativeLocation _needle02_2) (Math|Rotator|MakeRotator 1.8e+02 (- (.pitch (Variables|Default|GetNeedle02%20Relative)) 1e+01) 1.8e+02) false false 0.2 false)
          (Variables|Default|SetNeedle02%20Relative (Math|Rotator|MakeRotator 1.8e+02 (- (.pitch (Variables|Default|GetNeedle02%20Relative)) 1e+01) 1.8e+02)))))))

(event Custom|Switch%2003
  (bind _needle01 (Variables|Default|GetNeedle01))
  (bind _needle02 (Variables|Default|GetNeedle02))
  (bind _needle01_2 (Variables|Default|GetNeedle01))
  (bind _needle02_2 (Variables|Default|GetNeedle02))
  (if (Variables|Default|GetSwitch03On)
    (Utilities|FlowControl|Sequence
      (:then_0
        (Components|MoveComponentTo _needle01 (Variables|/Script/Engine.SceneComponent|GetRelativeLocation _needle01) (Math|Rotator|MakeRotator 1.8e+02 (- (.pitch (Variables|Default|GetNeedle01Relative)) -35.0) 1.8e+02) false false 0.2 false)
        (Variables|Default|SetNeedle01Relative (Math|Rotator|MakeRotator 1.8e+02 (- (.pitch (Variables|Default|GetNeedle01Relative)) -35.0) 1.8e+02)))
      (:then_1
        (Components|MoveComponentTo _needle02 (Variables|/Script/Engine.SceneComponent|GetRelativeLocation _needle02) (Math|Rotator|MakeRotator 1.8e+02 (- (.pitch (Variables|Default|GetNeedle02%20Relative)) -2e+01) 1.8e+02) false false 0.2 false)
        (Variables|Default|SetNeedle02%20Relative (Math|Rotator|MakeRotator 1.8e+02 (- (.pitch (Variables|Default|GetNeedle02%20Relative)) -2e+01) 1.8e+02))))
    (else
      (Utilities|FlowControl|Sequence
        (:then_0
          (Components|MoveComponentTo _needle01_2 (Variables|/Script/Engine.SceneComponent|GetRelativeLocation _needle01_2) (Math|Rotator|MakeRotator 1.8e+02 (- (.pitch (Variables|Default|GetNeedle01Relative)) 35.0) 1.8e+02) false false 0.2 false)
          (Variables|Default|SetNeedle01Relative (Math|Rotator|MakeRotator 1.8e+02 (- (.pitch (Variables|Default|GetNeedle01Relative)) 35.0) 1.8e+02)))
        (:then_1
          (Components|MoveComponentTo _needle02_2 (Variables|/Script/Engine.SceneComponent|GetRelativeLocation _needle02_2) (Math|Rotator|MakeRotator 1.8e+02 (- (.pitch (Variables|Default|GetNeedle02%20Relative)) 2e+01) 1.8e+02) false false 0.2 false)
          (Variables|Default|SetNeedle02%20Relative (Math|Rotator|MakeRotator 1.8e+02 (- (.pitch (Variables|Default|GetNeedle02%20Relative)) 2e+01) 1.8e+02)))))))

(event Custom|Answer
  (bind _returnvalue (Game|GetPlayerCharacter 0))
  (bind _returnvalue_2 (Game|GetPlayerController 0))
  (if (and (Variables|Default|GetSwitch02On) (Variables|Default|GetSwitch03On))
    (if (not (Variables|Default|GetSwitch01On))
      (if (not (Variables|Default|GetSwitch04On))
        (Game|Player|SetViewTargetwithBlend _returnvalue_2 _returnvalue 1.0 "VTBlend_Linear" 0.0 false)
        (Variables|/Script/Engine.PlayerController|SetbShowMouseCursor _returnvalue_2 false)
        (Variables|/Script/Engine.PlayerController|SetbEnableClickEvents _returnvalue_2 false)
        (Collision|SetActorEnableCollision false)
        (Input|SetInputModeGameOnly _returnvalue_2 false)
        (Input|EnableInput _returnvalue _returnvalue_2)
        (bind _newtrack_0 (Timeline|Door%20Anim Play)
          (:Update
            (Transformation|SetRelativeRotation (Variables|Default|GetScene) (Math|Rotator|MakeRotator 0.0 0.0 _newtrack_0) false false)))))))

(event EventInteract
  (bind _returnvalue (Game|GetPlayerController 0))
  (Class|WidgetBlueprintLibrary|SetFocustoGameViewport)
  (Utilities|FlowControl|DoOnce false :!label _label
    (:Completed
      (Utilities|FlowControl|Sequence
        (:then_0
          (bind _asbp_first_person_character (Utilities|Casting|CastToBP_FirstPersonCharacter (Game|GetPlayerCharacter 0)))
          (Rendering|SetActorHiddenInGame _asbp_first_person_character true)
          (Input|DisableInput _asbp_first_person_character _returnvalue)
          (Game|Player|SetViewTargetwithBlend _returnvalue self 0.25 "VTBlend_Linear" 0.0 false)
          (Rendering|SetVisibility (Variables|Default|GetWidget) false false)
          (Variables|/Script/Engine.PlayerController|SetbEnableClickEvents _returnvalue true)
          (Variables|/Script/Engine.PlayerController|SetbShowMouseCursor _returnvalue true))
        (:then_1
          (Utilities|FlowControl|Delay 1.0)
          (goto _label Reset))))))

(event EventBeginPlay
  (Variables|Default|SetNeedle01Relative (Variables|/Script/Engine.SceneComponent|GetRelativeRotation (Variables|Default|GetNeedle01)))
  (Variables|Default|SetNeedle02%20Relative (Variables|/Script/Engine.SceneComponent|GetRelativeRotation (Variables|Default|GetNeedle02))))

(fn ConstructionScript
  (|CallParentFunction))