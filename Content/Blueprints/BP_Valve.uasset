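; BP_Valve is an interactable valve that plays a turning animation when used.
; Interact destroys StaticMesh1 and plays the Animation timeline, whose Valve track drives the Valve component's relative pitch.
; The timeline update also disables actor collision, and a separate ValveActivate event turns collision back on.
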(event Custom|Valve%20Activate
  (Collision|SetActorEnableCollision true))

(event EventInteract
  (Components|DestroyComponent (Variables|Default|GetStaticMesh1))
  (bind _valve (Timeline|Animation Play)
    (:Update
      (Transformation|SetRelativeRotation (Variables|Default|GetValve) (Math|Rotator|MakeRotator 0.0 _valve 0.0) false false)
      (Collision|SetActorEnableCollision false))))

(fn ConstructionScript
  (|CallParentFunction))