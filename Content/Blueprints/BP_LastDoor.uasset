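; BP_LastDoor is an interactable door that opens once the player enters the correct code in a keypad-style widget.
; Interacting creates the UI_Codedore widget with its password, disables player character input and shows the mouse cursor.
; A looping timer set to the frame delta polls the widget's password flag, then a DoOnce fires a timeline that rotates the Scene component's yaw.
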(event Custom|Check
  (if (Variables|/Game/Blueprints/UI/UI_Codedore.UI_Codedore_C|GetbIsRightPassword (Variables|Default|GetNewVar))
    (Utilities|FlowControl|DoOnce false
      (:Completed
        (bind _newtrack_0 (Timeline|Timeline Play)
          (:Update
            (Transformation|SetRelativeRotation (Variables|Default|GetScene) (Math|Rotator|MakeRotator 0.0 0.0 _newtrack_0) false false)))))))

(event EventInteract
  (bind _returnvalue (Game|GetPlayerController 0))
  (bind _returnvalue_2 (UserInterface|CreateWidget "/Game/Blueprints/UI/UI_Codedore.UI_Codedore_C"))
  (bind _output_get (Variables|Default|SetNewVar _returnvalue_2))
  (UserInterface|Viewport|AddtoViewport _returnvalue_2 0)
  (Input|DisableInput (Game|GetPlayerCharacter 0) _returnvalue)
  (Variables|/Script/Engine.PlayerController|SetbShowMouseCursor _returnvalue true)
  (Utilities|Time|SetTimerbyEvent (delegate Custom|Check) (Utilities|Time|GetWorldDeltaSeconds) true))

(fn ConstructionScript
  (|CallParentFunction))