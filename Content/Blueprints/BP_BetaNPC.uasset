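; BP_BetaNPC is an interactable NPC that moves the player's view from the first-person character to itself and back.
; Interact hides the character, disables its input, blends the camera to the NPC, hides a widget and enables click events, guarded by a DoOnce that resets after a delay.
; Clicking its Plane component unhides the character, restores input and blends the view back, leaving the widget hidden.
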(event OnClicked(Plane)
  (params (TouchedComponent :type Primitive%20Component%20Object%20Reference) (ButtonPressed :type Key%20Structure :default "None"))
  (bind _returnvalue (Game|GetPlayerCharacter 0))
  (bind _returnvalue_2 (Game|GetPlayerController 0))
  (bind _asbp_first_person_character (Utilities|Casting|CastToBP_FirstPersonCharacter _returnvalue))
  (Rendering|SetActorHiddenInGame _asbp_first_person_character false)
  (Input|EnableInput _returnvalue _returnvalue_2)
  (Game|Player|SetViewTargetwithBlend _returnvalue_2 _returnvalue 0.25 "VTBlend_Linear" 0.0 false))

(event EventInteract
  (bind _returnvalue (Game|GetPlayerController 0))
  (Class|WidgetBlueprintLibrary|SetFocustoGameViewport)
  (Utilities|FlowControl|DoOnce false :!label _label
    (:Completed
      (Utilities|FlowControl|Sequence
        (:then_0
          (bind _asbp_first_person_character (Utilities|Casting|CastToBP_FirstPersonCharacter (Game|GetPlayerCharacter 0)))
          (Rendering|SetActorHiddenInGame _asbp_first_person_character true)
          (Input|DisableInput _asbp_first_person_character _returnvalue)
          (Game|Player|SetViewTargetwithBlend _returnvalue self 0.25 "VTBlend_Linear" 0.0 false)
          (Rendering|SetVisibility (Variables|Default|GetWidget) false false)
          (Variables|/Script/Engine.PlayerController|SetbEnableClickEvents _returnvalue true))
        (:then_1
          (Utilities|FlowControl|Delay 1.0)
          (goto _label Reset))))))

(fn ConstructionScript
  (|CallParentFunction))