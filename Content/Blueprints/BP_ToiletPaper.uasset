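; Toilet paper pickup actor that records when it has been collected through a HaveToiletPaper flag.
; It starts with collision disabled, and a Spawn event applies the toilet paper material without re-enabling collision.
; Interact sets the flag, swaps the mesh to an invisible material and disables collision, hiding the actor rather than destroying it.
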(event Custom|Spawn
  (Rendering|Material|SetMaterial (Variables|Default|GetStaticMesh) 0 "/Game/Materials/M_ToiletPaper.M_ToiletPaper"))

(event EventInteract
  (Rendering|Material|SetMaterial (Variables|Default|GetStaticMesh) 0 "/Game/Materials/M_Invisible.M_Invisible")
  (Variables|Default|SetHave%20Toilet%20Paper true)
  (Collision|SetActorEnableCollision false))

(event EventBeginPlay
  (Collision|SetActorEnableCollision false))

(fn ConstructionScript
  (|CallParentFunction))